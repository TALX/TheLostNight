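; Rifle weapon (Gewehr) that fires projectile actors and tracks clip and reserve ammo.
; Fire spends a round and spawns two Jagdgwehr_Base actors, one at its own "shot" socket and a scaled-down one at the player's rifle socket, plus a muzzle sound, without checking ammo.
; Reload overwrites the clip from reserve, deducting a full clip regardless of rounds left.
; A pickup-style MaxAmmo function adds a fixed amount to reserve.
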(event Custom|Fire
  (Game|SpawnActorfromClass "/Game/Assets/Blueprints/Waffen/Jagdgwehr_Base.Jagdgwehr_Base_C" (Transformation|GetSocketTransform (Variables|Default|GetSkeletalMesh1) "shot" "RTS_World") "Undefined" 0 0)
  (Variables|Default|Setammo (- (Variables|Default|Getammo) 1))
  (bind _asplayer (Utilities|Casting|CastToPlayer (Game|GetPlayerCharacter 0)))
  (bind _returnvalue (Game|SpawnActorfromClass "/Game/Assets/Blueprints/Waffen/Jagdgwehr_Base.Jagdgwehr_Base_C" (Math|Transform|MakeTransform (Transformation|GetSocketLocation (Variables|Gewehr_BP_C|GetSkeletalMesh1 (Variables|/Game/Player/Player.Player_C|GetGewehr _asplayer)) "shot") (Transformation|GetSocketRotation (Variables|Gewehr_BP_C|GetSkeletalMesh1 (Variables|/Game/Player/Player.Player_C|GetGewehr _asplayer)) "shot")) "Undefined" 0 0))
  (Transformation|SetWorldScale3D (Variables|/Script/Engine.Actor|GetRootComponent _returnvalue) "0.100000,0.100000,0.100000")
  (Audio|SpawnSoundatLocation "/Game/soundEffects/gun/Rifle_Sound_Effect__Very_High_Quality_.Rifle_Sound_Effect__Very_High_Quality_" (Transformation|GetSocketLocation (Variables|Default|GetSkeletalMesh1) "muzzle")))

(fn ConstructionScript)

(fn Reload
  (if (not (== (Variables|Default|Getammo) (Variables|Default|GetClipSize)))
    (if (> (Variables|Default|GetMaxAmmo) (Variables|Default|GetClipSize))
      (Variables|Default|Setammo (Variables|Default|GetClipSize))
      (Variables|Default|SetMaxAmmo (- (Variables|Default|GetMaxAmmo) (Variables|Default|GetClipSize)))
      (else
        (Variables|Default|Setammo (Variables|Default|GetMaxAmmo))
        (Variables|Default|SetMaxAmmo 0)))))

(fn MaxAmmo
  (Variables|Default|SetMaxAmmo (+ (Variables|Default|GetMaxAmmo) 8)))