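; Collectible pickup actor that the player gathers by touching it.
; When its Box component is overlapped, it destroys itself, then casts the overlapping actor to Player and increments that player's Collectives count.
; Any overlapping actor destroys it, even if it is not a Player.
; A disconnected branch that would show a Win widget never runs.
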(event OnComponentBeginOverlap(Box)
  (params (OverlappedComponent :type Primitive%20Component%20Object%20Reference) (OtherActor :type Actor%20Object%20Reference) (OtherComp :type Primitive%20Component%20Object%20Reference) (OtherBodyIndex :type Integer) (bFromSweep :type Boolean) (SweepResult :type Hit%20Result%20Structure%20%28by%20ref%29))
  (Actor|DestroyActor)
  (bind _asplayer (Utilities|Casting|CastToPlayer OtherActor))
  (Variables|/Game/Player/Player.Player_C|SetCollectives _asplayer (+ (Variables|/Game/Player/Player.Player_C|GetCollectives _asplayer) 1)))

(event EventBeginPlay)

(event Collision|EventActorBeginOverlap
  (params (OtherActor :type Actor%20Object%20Reference)))

(event EventTick
  (params (DeltaSeconds :type Float%20%28single-precision%29))
  (if true
    _))

(fn ConstructionScript)